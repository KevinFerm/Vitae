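; Stat component that tracks life and mana, starting both at maximum on initialization and regenerating them over time.
; Tick drives timers that add amplified amounts plus bonuses at scaled intervals, refreshing per-second display strings.
; Regeneration requires its toggle and skips any step that would exceed the maximum rather than clamping.
; GiveDamage forwards to another Stat's TakeDamage, which ignores damage greater than current life.
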(event EventTick
  (params (DeltaSeconds :type Float%20%28single-precision%29))
  (CallFunction|Generation DeltaSeconds))

(event EventInitializeComponent
  (Variables|PrimaryStats|SetCurrent%20Life (Variables|PrimaryStats|GetMax%20Life))
  (Variables|PrimaryStats|SetCurrent%20Mana (Variables|PrimaryStats|GetMax%20Mana)))

(fn LifeGeneration
  (params (Time :type Float%20%28single-precision%29))
  (bind _life_regeneration_bonus (Variables|AdditionalStats|GetLife%20Regeneration%20Bonus))
  (bind _life_amplifier (Variables|AdditionalStats|GetLife%20Amplifier))
  (bind _life_regeneration (Variables|AdditionalStats|GetLife%20Regeneration))
  (bind _life_regeneration_speed (Variables|AdditionalStats|GetLife%20Regeneration%20Speed))
  (bind _life_regeneration_speed_amplifier (Variables|AdditionalStats|GetLife%20Regeneration%20Speed%20Amplifier))
  (bind _returnvalue (* _life_regeneration _life_amplifier))
  (bind _returnvalue_2 (* _life_regeneration_speed _life_regeneration_speed_amplifier))
  (bind _returnvalue_3 (Math|Float|Floor _returnvalue))
  (Variables|Default|SetLife%20Timer (+ Time (Variables|Default|GetLife%20Timer)))
  (if (>= (Variables|Default|GetLife%20Timer) _returnvalue_2)
    (Variables|Display|SetLife%20per%20Sec (Utilities|String|ToString(Float) (/ (Math|Conversions|ToFloat(Integer) (+ _life_regeneration_bonus _returnvalue_3)) _returnvalue_2)))
    (Variables|Default|SetLife%20Timer 0.0)
    (if (and (<= (+ (Variables|PrimaryStats|GetCurrent%20Life) _returnvalue_3 _life_regeneration_bonus) (Variables|PrimaryStats|GetMax%20Life)) (Variables|Default|GetLife%20Generation%20Toggle))
      (Variables|PrimaryStats|SetCurrent%20Life (+ (Variables|PrimaryStats|GetCurrent%20Life) _returnvalue_3 _life_regeneration_bonus)))))

(fn ManaGeneration
  (params (Timer :type Float%20%28single-precision%29 :default 0.0))
  (bind _mana_regeneration_bonus (Variables|AdditionalStats|GetMana%20Regeneration%20Bonus))
  (bind _mana_regeneration (Variables|AdditionalStats|GetMana%20Regeneration))
  (bind _mana_amplifier (Variables|AdditionalStats|GetMana%20Amplifier))
  (bind _mana_regeneration_speed (Variables|AdditionalStats|GetMana%20Regeneration%20Speed))
  (bind _mana_regeneration_speed_amplifier (Variables|AdditionalStats|GetMana%20Regeneration%20Speed%20Amplifier))
  (bind _returnvalue (* _mana_regeneration _mana_amplifier))
  (bind _returnvalue_2 (* _mana_regeneration_speed _mana_regeneration_speed_amplifier))
  (bind _returnvalue_3 (Math|Float|Floor _returnvalue))
  (Variables|Default|SetMana%20Timer (+ Timer (Variables|Default|GetMana%20Timer)))
  (if (>= (Variables|Default|GetMana%20Timer) _returnvalue_2)
    (Variables|Default|SetMana%20Timer 0.0)
    (Variables|Display|SetMana%20per%20Sec (Utilities|String|ToString(Float) (/ (Math|Conversions|ToFloat(Integer) (+ _mana_regeneration_bonus _returnvalue_3)) _returnvalue_2)))
    (if (and (<= (+ (Variables|PrimaryStats|GetCurrent%20Mana) _returnvalue_3 _mana_regeneration_bonus) (Variables|PrimaryStats|GetMax%20Mana)) (Variables|Default|GetMana%20Generation%20Toggle))
      (Variables|PrimaryStats|SetCurrent%20Mana (+ (Variables|PrimaryStats|GetCurrent%20Mana) _returnvalue_3 _mana_regeneration_bonus)))))

(fn TakeDamage
  (params (Damage :type Integer :default 0))
  (if (>= (Variables|PrimaryStats|GetCurrent%20Life) Damage)
    (Variables|PrimaryStats|SetCurrent%20Life (- (Variables|PrimaryStats|GetCurrent%20Life) Damage))))

(fn GiveDamage
  (params (Target :type Actor%20Object%20Reference) (Damage :type Integer :default 0))
  (bind _asstat (Utilities|Casting|CastToStat Target))
  (CallFunction|TakeDamage _asstat Damage))

(fn Generation
  (params (time :type Float%20%28single-precision%29))
  (Variables|Display|SetLife%20per%20Sec (Utilities|String|ToString(Float) (/ (Math|Conversions|ToFloat(Integer) (+ (Variables|AdditionalStats|GetLife%20Regeneration%20Bonus) (Math|Float|Floor (* (Variables|AdditionalStats|GetLife%20Regeneration) (Variables|AdditionalStats|GetLife%20Amplifier))))) (* (Variables|AdditionalStats|GetLife%20Regeneration%20Speed) (Variables|AdditionalStats|GetLife%20Regeneration%20Speed%20Amplifier)))))
  (Variables|Display|SetMana%20per%20Sec (Utilities|String|ToString(Float) (/ (Math|Conversions|ToFloat(Integer) (+ (Variables|AdditionalStats|GetMana%20Regeneration%20Bonus) (Math|Float|Floor (* (Variables|AdditionalStats|GetMana%20Regeneration) (Variables|AdditionalStats|GetMana%20Amplifier))))) (* (Variables|AdditionalStats|GetMana%20Regeneration%20Speed) (Variables|AdditionalStats|GetMana%20Regeneration%20Speed%20Amplifier)))))
  (CallFunction|LifeGeneration time)
  (CallFunction|ManaGeneration time))