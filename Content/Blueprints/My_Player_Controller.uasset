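; Player controller Blueprint that toggles the mouse cursor and click events together.
; Right mouse button flips the state on both press and release, acting as a hold, while releasing M flips it as a persistent toggle.
; An unconnected cast to MyCharacter, an unused direction transform from its LookingAtActor, and an empty macro do nothing.
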(event Input|MouseEvents|RightMouseButton
  ;[1 1 1] Toggle Mouse
  (:Pressed
    (Variables|Default|SetbEnableClickEvents (not (Variables|Default|GetbShowMouseCursor)) :!label _label)
    (Variables|Default|SetbShowMouseCursor (not (Variables|Default|GetbShowMouseCursor))))
  (:Released
    (goto _label)))

(event Input|KeyboardEvents|M
  ;[1 1 1] Toggle Mouse
  (:Released
    (Variables|Default|SetbEnableClickEvents (not (Variables|Default|GetbShowMouseCursor)))
    (Variables|Default|SetbShowMouseCursor (not (Variables|Default|GetbShowMouseCursor)))))

(fn ConstructionScript)