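; A HUD Blueprint that draws a debug text overlay of the player transform, mouse position and hit box state.
; DrawHUD stores screen size and mouse coordinates, then prints them alongside the last hovered and pressed box names, except screen size.
; Hit box events update those names, and ending cursor-over clears both.
; A minimap rectangle and texture draw exists but is disconnected, and no hit boxes are added here.
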(event EventDrawHUD
  (params (SizeX :type Integer) (SizeY :type Integer))
  (bind _returnvalue (Game|GetPlayerController 0))
  (bind (_locationx _locationy) (Game|Player|GetMousePosition _returnvalue))
  ;[1 1 1] Debug Player
  (Variables|Default|SetScreen_X SizeX)
  (Variables|Default|SetScreen_Y SizeY)
  (HUD|DrawText (Utilities|String|Append "Player: " (Utilities|String|ToString(Transform) (Transformation|GetActorTransform (Game|Player|GetPlayerPawn 0)))) "(R=1.000000,G=1.000000,B=1.000000,A=1.000000)" 0.0 0.0 0 1.0 false)
  ;[1 1 1] Debug Mouse
  (Variables|Default|SetMouse_Y _locationy)
  (Variables|Default|SetMouse_X _locationx)
  (HUD|DrawText (Utilities|String|Append "Mouse: " (Utilities|String|Append (Utilities|String|BuildString(Float) "" "" _locationx) (Utilities|String|BuildString(Float) ", " "" _locationy))) "(R=1.000000,G=1.000000,B=1.000000,A=1.000000)" 0.0 12.0 0 1.0 false)
  ;[1 1 1] Debug Last Hit Box
  (HUD|DrawText (Utilities|String|Append "Box over: " (Variables|Default|GetLast%20Over)) "(R=1.000000,G=1.000000,B=1.000000,A=1.000000)" 0.0 36.0 0 1.0 false)
  ;[1 1 1] Debug Last Hit Box
  (HUD|DrawText (Utilities|String|Append "Box press: " (Variables|Default|GetLast%20Press'd)) "(R=1.000000,G=1.000000,B=1.000000,A=1.000000)" 0.0 24.0 0 1.0 false))

(event EventHitBoxClick
  (params (BoxName :type Name :default "None"))
  ;[1 1 1] Hit Box Events
  (Variables|Default|SetLast%20Press'd (Utilities|String|ToString(Name) BoxName)))

(event EventHitBoxBeginCursorOver
  (params (BoxName :type Name :default "None"))
  ;[1 1 1] Hit Box Events
  (Variables|Default|SetLast%20Over (Utilities|String|ToString(Name) BoxName)))

(event EventHitBoxEndCursorOver
  (params (BoxName :type Name :default "None"))
  ;[1 1 1] Hit Box Events
  (Variables|Default|SetLast%20Over "")
  (Variables|Default|SetLast%20Press'd ""))

(event EventHitBoxRelease
  (params (BoxName :type Name :default "None"))
  ;[1 1 1] Hit Box Events
  (Variables|Default|SetLast%20Press'd ""))

(fn ConstructionScript)