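; Death zone actor that, while Active, gradually heats toward red over a set Time and then flags itself as Evil.
; Tick raises Red to full, then lowers Green, pushing the color to the material's "Main Color" only during that second phase.
; The construction script applies the Size scale and creates dynamic Hex material instances on two meshes, keeping only the StaticMesh one for color updates.
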(event EventTick
  (params (DeltaSeconds :type Float%20%28single-precision%29))
  (bind _time (Variables|Default|GetTime))
  (bind _returnvalue (/ DeltaSeconds _time))
  (bind _returnvalue_2 (/ _returnvalue 2.0))
  (if (Variables|Default|GetActive)
    (if (<= (Variables|Color|GetRed) 1.0)
      (Variables|Color|SetRed (+ (Variables|Color|GetRed) _returnvalue_2))
      (elif (>= (Variables|Color|GetGreen) 0.0)
        (Variables|Color|SetGreen (- (Variables|Color|GetGreen) _returnvalue_2))
        (Rendering|Material|SetVectorParameterValue (Variables|Default|GetMaterial) "Main Color" (Utilities|Struct|MakeLinearColor (Variables|Color|GetRed) (Variables|Color|GetGreen) 0.0 1.0) :!class /Script/Engine.MaterialInstanceDynamic)
        (if (and (>= (Variables|Color|GetRed) 1.0) (<= (Variables|Color|GetGreen) 0.0))
          (Variables|Default|SetEvil true))))))

(event EventBeginPlay)

(fn ConstructionScript
  (bind _returnvalue (Rendering|Material|CreateDynamicMaterialInstance (Variables|Default|GetHex) 0 "/Game/Materials/Param/Hex.Hex" :!class /Script/Engine.PrimitiveComponent))
  (Variables|Default|SetMaterial _returnvalue)
  (bind _returnvalue_2 (Rendering|Material|CreateDynamicMaterialInstance (Variables|Default|GetStaticMesh) 0 "/Game/Materials/Param/Hex.Hex" :!class /Script/Engine.PrimitiveComponent))
  (Variables|Default|SetMaterial _returnvalue_2)
  (Transformation|SetWorldScale3D (Math|Conversions|ToVector(Float) (Variables|Default|GetSize))))