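; Spell-casting component that lets its owner aim and cast spells from a list, governed by mana, cooldowns and cast times.
; Holding an action previews line or area targeting with short-lived decals redrawn each Tick; cone and channel handling are stubs.
; Release checks cooldown and mana, then starts a cast timer that movement beyond the Focus tolerance cancels.
; Completion spends mana, spawns the spell actor at the owner, passes Power and LifeSpan, and starts its cooldown.
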(event Custom|Set%20Cast%20Timer
  (bind _spell_list (Variables|Default|GetSpell%20List))
  (bind _selected_spell (Variables|Default|GetSelected%20Spell))
  (bind _item (Utilities|Array|Get(acopy) _spell_list _selected_spell))
  ;[1 1 1] Cast Setup
  (if (and (<= (Utilities|Array|Get(acopy) (Variables|Default|GetCurrent%20Cooldown) _selected_spell) 0.0) (>= (Variables|Default|GetCurrent%20Mana) (.mana _item)))
    (Variables|Default|SetMana%20Generation%20Toggle false)
    (Variables|Default|SetCast%20Time (.casttime _item))
    (Variables|Cast|SetCast true)
    (Development|PrintString "Casting")
    (else
      (Development|PrintString "Unable to Cast"))))

(event Custom|Spell%20Trigger
  (bind _spell_list (Variables|Default|GetSpell%20List))
  (bind _selected_spell (Variables|Default|GetSelected%20Spell))
  (bind _item (Utilities|Array|Get(acopy) _spell_list _selected_spell))
  ;[1 1 1] Spell Triggerd
  (Variables|Default|SetCurrent%20Mana (- (Variables|Default|GetCurrent%20Mana) (.mana _item)))
  (bind _returnvalue (Game|SpawnActorfromClass (.magic_bp _item) (Math|Conversions|ToTransform(Vector) (Transformation|GetActorLocation (Components|GetOwner))) false 0))
  (Development|PrintString "Hello")
  (Variables|/Game/Blueprints/Spell.Spell_C|SetPower (Utilities|Array|Get(acopy) (Actor|GetComponentsByClass _returnvalue "/Game/Blueprints/Spell.Spell_C")) (.power _item))
  (Variables|/Game/Blueprints/Spell.Spell_C|SetLife%20Span (Utilities|Array|Get(acopy) (Actor|GetComponentsByClass _returnvalue "/Game/Blueprints/Spell.Spell_C")) (.lifespan _item))
  (Utilities|Array|SetArrayElem (Variables|Default|GetCurrent%20Cooldown) (Variables|Default|GetSelected%20Spell) (.cooldown _item)))

(event Custom|Set%20Target%20Type
  (bind _spell_list (Variables|Default|GetSpell%20List))
  (bind _selected_spell (Variables|Default|GetSelected%20Spell))
  (bind _item (Utilities|Array|Get(acopy) _spell_list _selected_spell))
  (bind _returnvalue (Math|Conversions|ToVector(Float) (.area_of_effect_size _item)))
  (bind _x (Math|Vector|BreakVector _returnvalue))
  (switch Utilities|FlowControl|Switch|Switchonenum_magic_target (.area_of_effect _item)
    (:NewEnumerator0
      (Class|GameplayStatics|SpawnDecalAttached "/Game/Props/Materials/barrel.barrel" (Math|Vector|MakeVector _x 1e+01 64.0) (VehicleSound|GetRootComponent (Components|GetOwner)) "None" (Math|Vector|MakeVector _x 0.0 -96.0) "0.000000,90.000000,0.000000" "KeepRelativeOffset" 0.001))
    (:NewEnumerator3
      (Class|GameplayStatics|SpawnDecalAttached 0 "0, 0, 0" 0 "None" "0, 0, 0" "0, 0, 0" "KeepRelativeOffset" 0.0))
    (:NewEnumerator1
      (bind _outhit (Collision|LineTraceByChannel "0, 0, 0" "0, 0, 0" "TraceTypeQuery1" false 0 "None"))
      (Rendering|Decal|SpawnDecalatLocation "/Game/Characters/Material/lambert4.lambert4" _returnvalue (.location _outhit) "0, 0, 0" 0.001))))

(event Custom|Channel
  (if (.channel (Utilities|Array|Get(acopy) (Variables|Default|GetSpell%20List) (Variables|Default|GetSelected%20Spell)))
    _))

(event Custom|Action%20Release
  (params (Action :type Integer :default 0))
  ;[1 1 1] Check Button Up and run selected attack
  (Variables|Default|SetSelected%20Spell Action)
  (CallFunction|SetCastTimer)
  (Variables|Default|SetDown false))

(event Custom|Action%20Press
  (params (Action :type Integer :default 0))
  ;[1 1 1] Check Button Down and charge selected attack
  (Variables|Default|SetSelected%20Spell Action)
  (CallFunction|Channel)
  (Variables|Default|SetDown true))

(event EventTick
  (params (DeltaSeconds :type Float%20%28single-precision%29))
  (bind _returnvalue (Components|GetOwner))
  (bind _returnvalue_2 (Transformation|GetVelocity _returnvalue))
  (if (Variables|Default|GetDown)
    (CallFunction|SetTargetType))
  (CallFunction|Generation DeltaSeconds)
  ;[1 1 1] Cooldown Timer
  (for (_array_element _array_index) (Variables|Default|GetCurrent%20Cooldown)
    (if (>= _array_element 0.0)
      (Utilities|Array|SetArrayElem (Variables|Default|GetCurrent%20Cooldown) _array_index (- _array_element DeltaSeconds))))
  ;[1 1 1] Cast Timer
  (if (Math|Boolean|ANDBoolean (Variables|Cast|GetCast) (> (Variables|Default|GetCast%20Time) 0.0) (Math|Float|NearlyEqual(Float) (+ (.x _returnvalue_2) (.y _returnvalue_2) (.z _returnvalue_2)) 0.0 (Math|Conversions|ToFloat(Integer) (Variables|Default|GetFocus))))
    (bind _output_get (Variables|Default|SetCast%20Time (- (Variables|Default|GetCast%20Time) DeltaSeconds)))
    (if (<= _output_get 0.0) ; If cast time is zero, trigger spell
      (CallFunction|SpellTrigger)
      (else
        (Development|PrintString (Utilities|String|ToString(Float) _output_get))))
    (else
      (Variables|Cast|SetCast false)
      (Variables|Default|SetMana%20Generation%20Toggle true))))

(event EventInitializeComponent
  ;[1 1 1] Init
  (Utilities|Array|Resize (Variables|Default|GetCurrent%20Cooldown) (Utilities|Array|Length (Variables|Default|GetSpell%20List))))