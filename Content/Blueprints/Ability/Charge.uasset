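; Charge ability Blueprint that launches the character in a dash when the 3 key is pressed, if grounded and off cooldown.
; It toggles ProjectileMovement, sets the capsule to zero rotation and applies a large impulse along that fixed world-forward direction, briefly disabling player input.
; After input returns, SprintDuration times the cooldown, then ProjectileMovement toggles again.
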(event Input|KeyboardEvents|3
  (bind _yaw (Class|KismetMathLibrary|BreakRot "0, 0, 0"))
  (bind _projectilemovement (Variables|Default|GetProjectileMovement))
  (bind _returnvalue (Class|KismetMathLibrary|MakeRot 0.0 _yaw 0.0))
  ;[0.685 0.4753 0.2772] Charge
  (:Pressed
    (if (not (Variables|Default|GetOnCoolDown))
      (if (not (AI|Components|NavMovement|IsFalling))
        (Input|DisableInput (Game|GetPlayerController 0))
        (Components|Activation|ToggleActive _projectilemovement)
        (Transformation|SetWorldRotation (Variables|Collision|GetCapsuleComponent) _returnvalue false)
        (Physics|AddImpulse (* (Math|Vector|GetForwardVector _returnvalue) 5e+06) false)
        (Utilities|FlowControl|Delay 0.3)
        (Input|EnableInput (Game|GetPlayerController 0))
        (Variables|Default|SetOnCoolDown true)
        (Utilities|FlowControl|Delay (Variables|Default|GetSprintDuration))
        (Components|Activation|ToggleActive _projectilemovement)
        (Variables|Default|SetOnCoolDown false)))))

(fn ConstructionScript)