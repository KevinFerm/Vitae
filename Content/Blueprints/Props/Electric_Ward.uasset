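; Electric_Ward is a short-lived prop that links to the other Electric_Ward actors with a particle beam.
; Every Tick it fetches all wards, finds itself in the array and aims its beam at the next ward's location.
; The last ward wraps around to the first, closing the chain into a loop.
; A Delay on the Tick path destroys the actor after five seconds.
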(event EventTick
  (params (DeltaSeconds :type Float%20%28single-precision%29))
  (bind _outactors (Actor|GetAllActorsOfClass "Electric_Ward_C"))
  (bind (_array_element _array_index) (Utilities|Array|ForEachLoopwithBreak _outactors :!label _label)
    (:LoopBody
      (if (== self _array_element)
        (if (== _array_index (Utilities|Array|LastIndex _outactors))
          (Variables|Default|SetIndex 0)
          (else
            (Variables|Default|SetIndex (+ _array_index 1))))
        (Class|ParticleSystemComponent|SetBeamTargetPoint 0 (Transformation|GetActorLocation (Utilities|Array|Get(acopy) _outactors (Variables|Default|GetIndex))))
        (goto _label Break)))
    (:Completed
      (Utilities|FlowControl|Delay 5.0)
      (Actor|DestroyActor))))

(fn ConstructionScript)