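; Teleport pad prop that sends an overlapping actor to the next Teleport in the level, wrapping from last to first.
; Trigger overlaps store the actor, and while one is present Tick runs a 1.5-second Delay, then finds the next pad via GetAllActorsOfClass.
; The destination pad's Teleport event moves the actor to its trigger, charging the player character 50 mana and refusing if short, while other actors travel free.
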(event OnComponentBeginOverlap(Trigger)
  (params (OtherActor :type Actor%20Object%20Reference) (OtherComp :type Primitive%20Component%20Object%20Reference) (OtherBodyIndex :type Integer) (bFromSweep :type Boolean) (SweepResult :type Hit%20Result%20Structure%20%28by%20ref%29))
  (Variables|Default|SetObjOn true)
  (Variables|Default|SetActorOn OtherActor))

(event OnComponentEndOverlap(Trigger)
  (params (OtherActor :type Actor%20Object%20Reference) (OtherComp :type Primitive%20Component%20Object%20Reference) (OtherBodyIndex :type Integer))
  (Variables|Default|SetObjOn false)
  (Variables|Default|SetActorOn 0))

(event Custom|Teleport
  (params (Actor :type Actor%20Object%20Reference))
  (bind _returnvalue (Game|GetPlayerCharacter 0))
  (if (== Actor _returnvalue)
    (bind _asmy_character (Utilities|Casting|CastToMyCharacter _returnvalue))
    (if (>= (- (Variables|/Game/Blueprints/MyCharacter.MyCharacter_C|GetCurrent%20Mana _asmy_character) 50) 0)
      (Variables|/Game/Blueprints/MyCharacter.MyCharacter_C|SetCurrent%20Mana _asmy_character (- (Variables|/Game/Blueprints/MyCharacter.MyCharacter_C|GetCurrent%20Mana _asmy_character) 50))
      (Transformation|Teleport Actor (Transformation|GetWorldLocation (Variables|Default|GetTrigger)) "0, 0, 0" :!label _label))
    (else
      (goto _label))))

(event EventTick
  (params (DeltaSeconds :type Float%20%28single-precision%29))
  (if (Variables|Default|GetObjOn)
    (Utilities|FlowControl|Delay 1.5)
    (bind _outactors (Actor|GetAllActorsOfClass "Teleport_C"))
    (bind (_array_element _array_index) (Utilities|Array|ForEachLoopwithBreak _outactors :!label _label)
      (:LoopBody
        (if (== _array_index (Utilities|Array|LastIndex _outactors))
          (Variables|Default|SetTeleportTo (Utilities|Array|Get(acopy) _outactors))
          (else
            (Variables|Default|SetTeleportTo (Utilities|Array|Get(acopy) _outactors (+ _array_index 1)))))
        (if (== _array_element self)
          (CallFunction|Teleport (Variables|Default|GetTeleportTo) (Variables|Default|GetActorOn))
          (goto _label Break))))))

(fn ConstructionScript)