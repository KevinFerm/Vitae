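; Barrel prop with configurable mesh and material that the player can target and launch with a push.
; Each tick it glows through custom depth while it is the player's LookingAtActor at mid range, otherwise clearing the glow and enabling gravity.
; While glowing, TriggerPuch applies a power-scaled impulse based on player and barrel rotations.
; High-velocity hits with Explode set only print a debug message.
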(event Custom|Trigger%20Puch
  (params (power :type Float%20%28single-precision%29))
  (bind _returnvalue (Game|GetPlayerCharacter 0))
  (bind _returnvalue_2 (Transformation|GetActorRotation))
  (bind _returnvalue_3 (Transformation|GetActorRotation _returnvalue))
  (bind _returnvalue_4 (Math|Rotator|Delta(Rotator) _returnvalue_3 _returnvalue_2))
  (bind _returnvalue_5 (Math|Vector|GetForwardVector _returnvalue_4))
  ;[1 1 1] Trigger Effect to make it FLYYYY
  (if (Variables|Default|GetGlow)
    (Physics|AddImpulseatLocation (Variables|Default|GetProjectile%20Movement) (Math|Transform|TransformDirection (Transformation|GetWorldTransform) (* _returnvalue_5 (* power 1e+05))) (Math|Transform|TransformDirection (Transformation|GetActorTransform _returnvalue) (* _returnvalue_5 1e+02)) "None")))

(event EventTick
  (params (DeltaSeconds :type Float%20%28single-precision%29))
  (bind _returnvalue (Game|GetPlayerCharacter 0))
  (bind _barrel (Variables|Default|GetBarrel))
  ;[1 1 1] Add Glow Effect if target
  (bind _asmy_character (Utilities|Casting|CastToMyCharacter _returnvalue))
  (if (== (Variables|/Game/Blueprints/MyCharacter.MyCharacter_C|GetLooking%20at%20Actor _asmy_character) self)
    (bind _returnvalue_2 (Transformation|GetDistanceTo _returnvalue))
    (Math|Float|CompareFloat _returnvalue_2 2.5e+02
      (:>
        (Math|Float|CompareFloat _returnvalue_2 1.5e+03
          (:>
            (Rendering|SetRenderCustomDepth _barrel false :!label _label)
            (Variables|Default|SetGlow false)
            (Physics|SetEnableGravity true))
          (:<
            (Rendering|SetRenderCustomDepth _barrel true)
            (Variables|Default|SetGlow true))))
      (:<
        (goto _label)))
    (else
      (goto _label))))

(event EventHit
  (params (MyComp :type Primitive%20Component%20Object%20Reference) (Other :type Actor%20Object%20Reference) (OtherComp :type Primitive%20Component%20Object%20Reference) (bSelfMoved :type Boolean) (HitLocation :type Vector :default "0, 0, 0") (HitNormal :type Vector :default "0, 0, 0") (NormalImpulse :type Vector :default "0, 0, 0") (Hit :type Hit%20Result%20Structure%20%28by%20ref%29))
  (bind _returnvalue (Transformation|GetVelocity Other))
  (bind _returnvalue_2 (Transformation|GetVelocity))
  (bind (_x _y _z) (Math|Vector|BreakVector _returnvalue))
  (bind (_x_2 _y_2 _z_2) (Math|Vector|BreakVector _returnvalue_2))
  (if (and (Math|Boolean|ORBoolean (> _x 4e+02) (> _y 4e+02) (> _z 4e+02) (> _x_2 4e+02) (> _y_2 4e+02) (> _z_2 4e+02)) (Variables|Default|GetExplode))
    (Development|PrintString "Hit Hard")))

(fn ConstructionScript
  (Components|StaticMesh|SetStaticMesh (Variables|Default|GetMesh))
  (Rendering|Material|SetMaterial 0 (Variables|Default|GetMaterial)))